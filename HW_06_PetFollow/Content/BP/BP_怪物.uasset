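; Monster character AI that wanders randomly, chases the player and performs timed melee attacks.
; A looping AI MoveTo chain from BeginPlay switches to chasing on pawn sensing or non-lethal bullet hits, and resumes wandering when the chase fails.
; On reaching the player it stops and briefly enables attack-area overlaps to deal damage.
; Lethal bullet damage ragdolls it, increments the game mode's kill count and destroys it after a delay.
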(event `self.感測元件.OnSeePawn`
  (params (Pawn :type "Pawn Object Reference"))
  (bind _charactermovement (`self.CharacterMovement`))
  (bind `_攻擊區域` (`self.攻擊區域`))
  ;[0 0.3277 1] 看到後保存玩家資訊
  (bind `_asbp_玩家控制` (cast `/Game/BP/BP_玩家控制` Pawn))
  (set `self.玩家控制` `_asbp_玩家控制`)
  (set `self.是否看到玩家` true :!label _label)
  (set `self.停留時間對大值` 0.0) ; 看到玩家後馬上往玩家前進
  (`/Engine/EditorBlueprintResources/StandardMacros.DoOnce` false ; 執行一次
    (:`Completed`
      ;[1 1 1] 判定有沒有看到玩家
      (if (`self.是否看到玩家`) :!label _label_2
        ;[0 0.3277 1] 看到玩家:追蹤玩家
        (`|AIMoveTo` self (0.0 0.0 0.0) (`self.玩家控制`) (`self.停止半徑`)
          (:`OnSuccess`
            ;[0.6667 0.1818 0.1319] 攻擊狀態
            (set `self.攻擊中` true)
            (set `CharacterMovementComponent.MaxWalkSpeed` 0.0 _charactermovement)
            (`KismetSystemLibrary.Delay` 1.4) ; 手舉起來的時間
            (set `PrimitiveComponent.bGenerateOverlapEvents` true `_攻擊區域`) ; 開啟碰撞
            (`KismetSystemLibrary.Delay` 0.2) ; 碰撞停留時間
            (set `PrimitiveComponent.bGenerateOverlapEvents` false `_攻擊區域`) ; 關閉碰撞
            (`KismetSystemLibrary.Delay` 2.7) ; 動畫完畢後
            (set `CharacterMovementComponent.MaxWalkSpeed` 500.0 _charactermovement)
            (set `self.攻擊中` false)
            (goto _label_2))
          (:`OnFail`
            (set `self.是否看到玩家` false)
            (set `self.停留時間對大值` 3.0) ; 恢復停留最大值為3
            (goto _label_2)))
        (else
          ;[0 0.3277 1] 沒看到玩家:隨機走動
          (`|AIMoveTo` self (`NavigationSystemV1.K2_GetRandomReachablePointInRadius` (`SceneComponent.K2_GetComponentLocation` (`self.CapsuleComponent`)) (`self.隨機走動半徑`) null null) null (`self.停止半徑`) ; AI 移動節點:移動到指定座標
            (:`then`
              ;[0 0.3277 1] 隨機停留
              (`KismetSystemLibrary.Delay` (* (`KismetMathLibrary.RandomFloat`) (`self.停留時間對大值`)))
              (goto _label_2))))))))

(event `self.ReceiveBeginPlay`
  (`|ExecutionSequence`
    (:`then_0`
      (goto _label_2))
    (:`then_1`
      ;[0.192 0.124 1] 取得遊戲模式
      (bind `_asbp_遊戲模式` (cast `/Game/BP/BP_遊戲模式` (`GameplayStatics.GetGameMode`)))
      (set `self.遊戲模式` `_asbp_遊戲模式`))))

(event `self.CapsuleComponent.OnComponentBeginOverlap`
  (params (OverlappedComponent :type "PrimitiveComponent Object Reference") (OtherActor :type "Actor Object Reference") (OtherComp :type "PrimitiveComponent Object Reference") (OtherBodyIndex :type Integer) (bFromSweep :type Boolean) (SweepResult :type "HitResult Structure (by ref)"))
  (bind `_遊戲模式` (`self.遊戲模式`))
  ;[1 0.5262 0.9736] 受傷與死亡
  (bind `_asbp_子彈` (cast `/Game/BP/BP_子彈` OtherActor))
  (bind `_是否死亡` (`self.受傷` (`/Game/BP/BP_子彈.目前武器傷害` `_asbp_子彈`)))
  (if `_是否死亡`
    (set `/Game/BP/BP_遊戲模式.擊殺的怪物數量` (+ (`/Game/BP/BP_遊戲模式.擊殺的怪物數量` `_遊戲模式`) 1) `_遊戲模式`)
    (`KismetSystemLibrary.Delay` 5.0)
    (`self.K2_DestroyActor`)
    (else
      (goto _label))))

(event `self.攻擊區域.OnComponentBeginOverlap`
  (params (OverlappedComponent :type "PrimitiveComponent Object Reference") (OtherActor :type "Actor Object Reference") (OtherComp :type "PrimitiveComponent Object Reference") (OtherBodyIndex :type Integer) (bFromSweep :type Boolean) (SweepResult :type "HitResult Structure (by ref)"))
  ;[0.6667 0.1818 0.1319] 攻擊區域判定與傳送傷害
  (bind `_asbp_玩家控制` (cast `/Game/BP/BP_玩家控制` OtherActor))
  (`/Game/BP/BP_玩家控制.受傷` `_asbp_玩家控制` (`self.怪物攻擊力`)))

(fn `UserConstructionScript`)

(fn `受傷`
  (params (`接受到的傷害` :type "Float (double-precision)"))
  (returns (`是否死亡` :type Boolean))
  ;[0.6667 0.1818 0.1319] 受傷
  (bind _output_get (set `self.血量` (- (`self.血量`) `接受到的傷害`)))
  (if (<= _output_get 0.0)
    ;[0.6667 0.1818 0.1319] 死亡
    (`PrimitiveComponent.SetSimulatePhysics` (`self.Mesh`) true) ; 模擬布偶效果
    (`PrimitiveComponent.SetCollisionEnabled` (`self.CapsuleComponent`) "NoCollision") ; 設定碰撞啟動:關閉膠囊碰撞避免產生太大碰撞
    (return true)
    (else
      (return false))))